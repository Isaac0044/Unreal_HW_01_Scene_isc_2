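; BP_武器 is a weapon Blueprint that handles automatic firing, magazine reloading and ammo pickup for the player.
; Holding the 開槍 input runs a Delay loop that spawns BP_子彈 at the muzzle socket with weapon damage and a flash, consuming ammo.
; Firing starts only if BP_玩家控制 is neither reloading nor sprinting.
; 換彈夾 refills the magazine from reserves, while 補充子彈 adds a magazine's worth to reserves, clamped to a maximum.
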(event Custom|換彈夾
  ;[0 1 0.171] 計算需補充子彈數
  (Variables|Default|Set要補充的子彈數量 (- (Variables|Default|Get彈夾尺寸) (Variables|Default|Get目前子彈數量))) ; 計算需補充子彈數量
  ;[0 1 0.3813] 判斷子彈總是是否>=要補充子彈數
  (if (>= (Variables|Default|Get總子彈數量) (Variables|Default|Get要補充的子彈數量))
    _
    (else
      ;[0 0.928 1] 子彈總數小於要補充子彈量
      (Variables|Default|Set要補充的子彈數量 (Variables|Default|Get總子彈數量))))
  ;[0.7471 1 0.1291] 目前子彈與總數更新
  (Variables|Default|Set目前子彈數量 (+ (Variables|Default|Get目前子彈數量) (Variables|Default|Get要補充的子彈數量))) ; 補充子彈數量
  (Variables|Default|Set總子彈數量 (- (Variables|Default|Get總子彈數量) (Variables|Default|Get要補充的子彈數量))) ; 扣除子彈總數
)

(event Custom|補充子彈
  ;[0.2154 1 0] 補充子彈
  (bind _output_get (Variables|Default|Set總子彈數量 (+ (Variables|Default|Get彈夾尺寸) (Variables|Default|Get總子彈數量)))) ; 子彈總數+彈夾尺寸
  (Variables|Default|Set總子彈數量 (Math|Integer|Clamp(Integer) _output_get 0 (Variables|Default|Get子彈上限))))

(event EventBeginPlay
  ;[0.3617 0.7085 1] 取得玩家資訊
  (bind _asbp_玩家控制 (Utilities|Casting|CastToBP_玩家控制 (Game|GetPlayerCharacter 0)))
  (Variables|Default|SetBP%20玩家控制 _asbp_玩家控制))

(event Input|ActionEvents|InputAction開槍
  (params (Key :type Key%20Structure :default "None"))
  (bind _武器模型 (Variables|Default|Get武器模型))
  (bind _bp_玩家控制 (Variables|Default|GetBP%20玩家控制))
  (bind _returnvalue (Transformation|GetSocketRotation _武器模型 "None"))
  ;[1 1 1] 開槍功能
  (:Pressed
    (if (and (not (Variables|/Game/BP/BP_玩家控制.BP_玩家控制_C|Get換彈夾 _bp_玩家控制)) (not (Variables|/Game/BP/BP_玩家控制.BP_玩家控制_C|Get衝刺 _bp_玩家控制))) ; 玩家不在換彈夾和衝刺中,才能開槍
      (Variables|Default|Set開槍中 true)
      (if (and (> (Variables|Default|Get目前子彈數量) 0) (Variables|Default|Get開槍中)) :!label _label ; 目前子彈>0才能開槍
        (bind _returnvalue_2 (Game|SpawnActorfromClass "/Game/BP/BP_子彈.BP_子彈_C" (Transformation|GetSocketTransform (Variables|Default|Get武器模型) "子彈插槽" "RTS_World") "Undefined" 0 0)) ; 生成子彈藍圖
        (Variables|/Game/BP/BP_子彈.BP_子彈_C|Set目前武器傷害 _returnvalue_2 (Variables|Default|Get武器傷害)) ; 將武器傷害傳給子彈
        (Effects|SpawnEmitteratLocation "/Game/InfinityBladeEffects/Effects/FX_Monsters/FX_Monster_Gruntling/Master/P_BackPack_MuzzleFlash.P_BackPack_MuzzleFlash" (Transformation|GetSocketLocation _武器模型 "子彈插槽") (Math|Rotator|MakeRotator (+ (.roll _returnvalue) 9e+01) (.pitch _returnvalue) (+ (.yaw _returnvalue) 9e+01)) "0.070000,0.070000,0.070000")
        (Variables|Default|Set目前子彈數量 (- (Variables|Default|Get目前子彈數量) 1))
        (Utilities|FlowControl|Delay (Variables|Default|Get開槍間隔))
        (goto _label))))
  (:Released
    (Variables|Default|Set開槍中 false)))

(fn ConstructionScript)