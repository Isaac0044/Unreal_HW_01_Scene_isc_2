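; Game mode Blueprint (遊戲模式) that runs a minutes-and-seconds countdown and records the monster kill target.
; BeginPlay counts actors tagged "怪物" (monster) into 需擊殺怪物數量 (monsters to kill).
; Tick feeds a one-second Delay as a makeshift timer, decrementing seconds and borrowing from minutes on underflow.
; When seconds underflow with no minutes left, it resets seconds to zero and pauses the game.
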(event EventTick
  (params (DeltaSeconds :type Float%20%28single-precision%29))
  ;[0.6137 1 0.3549] 倒數系統
  ;;[0.9092 1 0.09719] 每秒秒數減一
  (Utilities|FlowControl|Delay 1.0) ; 延遲
  (bind _output_get (Variables|Default|Set秒 (- (Variables|Default|Get秒) 1)))
  ;;[0 0.9849 1] 秒數歸0跳59
  (if (< _output_get 0) ; 判斷
    (Variables|Default|Set秒 59)
    ;;[0 0.2302 1] 分大於零分-1
    (if (> (Variables|Default|Get分) 0)
      (Variables|Default|Set分 (- (Variables|Default|Get分) 1))
      (else
        ;;[0.5474 0 1] 分等於0 秒等於59 秒歸零時暫停遊戲
        (if (== (Variables|Default|Get秒) 59)
          (Variables|Default|Set秒 0)
          (Game|SetGamePaused true))))))

(event EventBeginPlay
  ;[0.5018 1 0.2475] 取得貼有怪物標籤的所有物件並儲存數量
  (bind _outactors (Actor|GetAllActorswithTag "怪物"))
  (Variables|Default|Set需擊殺怪物數量 (Utilities|Array|Length _outactors)))

(fn ConstructionScript)